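; AI controller for the Minion enemy that runs BT_Enemy on possess and feeds perception results to its Blackboard.
; Sensing a "Player"-tagged actor cancels the timer and records line of sight, that actor, and the stimulus ReceiverLocation as last known location.
; Any other perception update starts a LineOfSightTimer countdown, which on expiry clears those keys, giving a delay before losing the target.
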(event `self.ReceivePossess`
  (params (PossessedPawn :type "Pawn Object Reference"))
  (`self.RunBehaviorTree` "/Game/Characters/Enemies/Behavior/BT_Enemy.BT_Enemy"))

(event `self.AIPerception.OnTargetPerceptionUpdated`
  (params (Actor :type "Actor Object Reference") (Stimulus :type "AIStimulus Structure"))
  (bind (_age _expirationage _strength _stimuluslocation _receiverlocation _tag _bsuccessfullysensed) (break `AIStimulus` Stimulus))
  (bind _blackboard (`self.Blackboard`))
  (if (and (`self.ActorHasTag` Actor "Player") _bsuccessfullysensed)
    (`KismetSystemLibrary.K2_ClearAndInvalidateTimerHandle` (`self.Enemy Timer`))
    (`BlackboardComponent.SetValueAsBool` _blackboard (`self.HasLineOfSight`) true)
    (`BlackboardComponent.SetValueAsObject` _blackboard (`self.EnemyActor`) Actor)
    (`BlackboardComponent.SetValueAsVector` _blackboard (`self.EnemyLastKnownLocation`) _receiverlocation)
    (else
      (bind _returnvalue (`KismetSystemLibrary.K2_SetTimerDelegate` (delegate `StartEnemyTimer`) (`self.LineOfSightTimer`)))
      (set `self.Enemy Timer` _returnvalue))))

(event `StartEnemyTimer`
  (bind _blackboard (`self.Blackboard`))
  (`BlackboardComponent.SetValueAsBool` _blackboard (`self.HasLineOfSight`) false)
  (`BlackboardComponent.SetValueAsObject` _blackboard (`self.EnemyActor`) null)
  (`BlackboardComponent.SetValueAsVector` _blackboard (`self.EnemyLastKnownLocation`) (0.0 0.0 0.0)))

(fn `UserConstructionScript`)