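; Player controller for Embercore that handles ability firing input and opening the pause menu.
; While Ability1 is held, Tick calls Shoot, which activates GA_Shoot from the player character's ability list through the player state's Ability System Component.
; P or Escape creates the PauseMenu widget once, then shows it, switches to UI-only input and pauses the game.
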(event `InputAction|Ability1`
  (params (Key :type "Key Structure"))
  (:`Pressed`
    (set `self.Ability1Held` true))
  (:`Released`
    (set `self.Ability1Held` false)))

(event `self.ReceiveTick`
  (params (DeltaSeconds :type "Float (single-precision)"))
  (if (`self.Ability1Held`)
    (`self.Shoot`)))

(event `Key|P`
  (params (Key :type "Key Structure"))
  (bind _pausemenureference (`self.PauseMenuReference`))
  (:`Pressed`
    (`/Engine/EditorBlueprintResources/StandardMacros.IsValid` (`self.PauseMenuReference`) :!label _label
      (:`Is Valid`
        _)
      (:`Is Not Valid`
        (bind _returnvalue (`|CreateWidget` "/Game/Embercore/UI/Menus/PauseMenu.PauseMenu_C"))
        (set `self.PauseMenuReference` _returnvalue)))
    (`WidgetBlueprintLibrary.SetInputMode_UIOnlyEx` self _pausemenureference)
    (`UserWidget.AddToViewport` _pausemenureference 0)
    (`GameplayStatics.SetGamePaused` true)))

(event `Key|Escape`
  (params (Key :type "Key Structure"))
  (:`Pressed`
    (goto _label)))

(fn `Shoot`
  (bind _asplayer_character (cast `PlayerCharacter` (`GameplayStatics.GetPlayerCharacter` 0)))
  (bind _characterabilities (`EmbercoreCharacter.CharacterAbilities` _asplayer_character))
  (`AbilitySystemComponent.TryActivateAbilityByClass` (`AbilitySystemBlueprintLibrary.GetAbilitySystemComponent` (`GameplayStatics.GetPlayerState` 0)) (`|GetArrayItem` _characterabilities (`KismetArrayLibrary.Array_Find` _characterabilities "/Game/Embercore/Player/Abilities/Shoot/GA_Shoot.GA_Shoot_C")) true))

(fn `UserConstructionScript`)