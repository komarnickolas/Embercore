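; Rifle projectile for Embercore that damages the character it overlaps, ignoring its instigator.
; Sphere and Collision overlaps share one handler, where only the server applies damage and either side destroys the projectile.
; A pawn line trace toward the victim recovers a hit result for the GAS effect context.
; The server then applies the damage effect spec plus a flat engine ApplyDamage.
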(event `self.Sphere.OnComponentBeginOverlap`
  (params (OverlappedComponent :type "PrimitiveComponent Object Reference") (OtherActor :type "Actor Object Reference") (OtherComp :type "PrimitiveComponent Object Reference") (OtherBodyIndex :type Integer) (bFromSweep :type Boolean) (SweepResult :type "HitResult Structure (by ref)"))
  (if (!= (stale `self.Collision.OnComponentBeginOverlap` OtherActor) (`self.GetInstigator`)) :!label _label
    (`/Engine/EditorBlueprintResources/ActorMacros.Switch Has Authority`
      (:`Authority`
        (bind _asembercore_character (cast `EmbercoreCharacter` (stale `self.Collision.OnComponentBeginOverlap` OtherActor))
          (:`then`
            (if (`KismetSystemLibrary.IsValid` _asembercore_character)
              (bind _outhits (`KismetSystemLibrary.LineTraceMultiForObjects` :`Start` (`self.K2_GetActorLocation`) :`End` (`self.K2_GetActorLocation` _asembercore_character) :`ObjectTypes` (`|MakeArray` "ObjectTypeQuery3" :!type "EObjectTypeQuery Enum") :`DrawTime` 2.0))
              (for _array_element _outhits
                (if (== (`.HitActor` (`GameplayStatics.BreakHitResult` _array_element)) _asembercore_character)
                  (set `self.FinalHit` _array_element)
                  (break)))
              (bind _returnvalue (`AbilitySystemBlueprintLibrary.GetEffectContext` (`self.DamageEffectSpecHandle`)))
              (`AbilitySystemBlueprintLibrary.EffectContextAddHitResult` _returnvalue (`self.FinalHit`))
              (`AbilitySystemComponent.BP_ApplyGameplayEffectSpecToSelf` (`AbilitySystemBlueprintLibrary.GetAbilitySystemComponent` _asembercore_character) (`self.DamageEffectSpecHandle`))
              (`GameplayStatics.ApplyDamage` _asembercore_character 10.0 null null "/Script/Engine.DamageType")
              (`self.K2_DestroyActor`)))
          (:`CastFailed`
            (`self.K2_DestroyActor` :!label _label_2))))
      (:`Remote`
        (goto _label_2)))))

(event `self.Collision.OnComponentBeginOverlap`
  (params (OverlappedComponent :type "PrimitiveComponent Object Reference") (OtherActor :type "Actor Object Reference") (OtherComp :type "PrimitiveComponent Object Reference") (OtherBodyIndex :type Integer) (bFromSweep :type Boolean) (SweepResult :type "HitResult Structure (by ref)"))
  (goto _label))

(fn `UserConstructionScript`)