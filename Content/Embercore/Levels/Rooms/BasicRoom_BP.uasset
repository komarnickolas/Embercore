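; BasicRoom_BP is an Embercore room that spawns Enemy_BP actors at random points inside itself when it becomes active.
; It binds OnRoomActive on Tick, and each event call passes a DoN gate capped by a seeded random count up to MaxEnemies, spawning one enemy.
; Spawn points come from the GameState's map node for the room's Index, scaled by floor tile size, using the GameState's shared random stream for the count.
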(event `self.ReceiveBeginPlay`)

(event `self.ReceiveTick`
  (params (DeltaSeconds :type "Float (single-precision)"))
  (add `self.OnRoomActive` (delegate `OnRoomActive_Event`)))

(event `OnRoomActive_Event`
  (set `self.Active` true)
  (bind _stream (`self.GetStream`))
  (`/Engine/EditorBlueprintResources/StandardMacros.Do N` (`KismetMathLibrary.RandomIntegerInRangeFromStream` 0 (`self.MaxEnemies`) _stream)
    (:`Exit`
      (bind _returnvalue (`self.GetRandomPoint`))
      (`|SpawnActorFromClass` "/Game/Embercore/Enemies/Enemy/Enemy_BP.Enemy_BP_C" (`KismetMathLibrary.MakeTransform` (`KismetMathLibrary.MakeVector` (.x _returnvalue) (.y _returnvalue) 90.0)) "AdjustIfPossibleButAlwaysSpawn" "OverrideRootScale" null null))))

(fn `GetCurrentMap`
  (returns (Map :type "DungeonMap Object Reference"))
  (bind _asembercore_game_state_bp (cast `/Game/Embercore/EmbercoreGameState_BP` (`GameplayStatics.GetGameState`)))
  (return (`EmbercoreGameState.Map` _asembercore_game_state_bp)))

(fn `GetRandomPoint`
  (returns (ReturnValue :type "Vector Structure"))
  (bind _map (`self.GetCurrentMap`))
  (bind _output (`self.GetSelfRoom`))
  (bind _returnvalue (`DungeonMap.GetRandomPointFrom` _map (`.Room` (break `SubDungeon` _output))))
  (return (`KismetMathLibrary.MakeVector` (* (.x _returnvalue) (`DungeonMap.FloorWidth` _map)) (* (.y _returnvalue) (`DungeonMap.FloorHeight` _map)))))

(fn `GetSelfRoom`
  (returns (Output :type "SubDungeon Structure (by ref)"))
  (bind _map (`self.GetCurrentMap`))
  (return (`|GetArrayItem` (`DungeonMap.Nodes` _map) (`self.Index`))))

(fn `GetStream`
  (returns (Stream :type "RandomStream Structure"))
  (bind _asembercore_game_state_bp (cast `/Game/Embercore/EmbercoreGameState_BP` (`GameplayStatics.GetGameState`)))
  (return (`EmbercoreGameState.Stream` _asembercore_game_state_bp)))

(fn `UserConstructionScript`)