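; Interactable tower actor that starts the event of the dungeon room that owns it.
; An overlap box toggles input on its interactable component as an EmbercorePlayer enters or leaves, always using player controller 0.
; On interact, it disables input, passes its owning DungeonRoom to the game state's start-room event, marks the room active and destroys itself.
; Timer and input-toggle events only print debug strings.
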(event `self.Box.OnComponentBeginOverlap`
  (params (OverlappedComponent :type "PrimitiveComponent Object Reference") (OtherActor :type "Actor Object Reference") (OtherComp :type "PrimitiveComponent Object Reference") (OtherBodyIndex :type Integer) (bFromSweep :type Boolean) (SweepResult :type "HitResult Structure (by ref)"))
  (cast `EmbercorePlayer` OtherActor)
  (`InteractableComponent.ToggleInput` (`self.InteractableComponent_BP`) (`GameplayStatics.GetPlayerController` 0) true))

(event `self.Box.OnComponentEndOverlap`
  (params (OverlappedComponent :type "PrimitiveComponent Object Reference") (OtherActor :type "Actor Object Reference") (OtherComp :type "PrimitiveComponent Object Reference") (OtherBodyIndex :type Integer))
  (cast `EmbercorePlayer` OtherActor)
  (`InteractableComponent.ToggleInput` (`self.InteractableComponent_BP`) (`GameplayStatics.GetPlayerController` 0) false))

(event `self.InteractableComponent_BP.OnInteractEvent`
  (`KismetSystemLibrary.PrintString` "Interact")
  (`InteractableComponent.ToggleInput` (`self.InteractableComponent_BP`) (`GameplayStatics.GetPlayerController` 0) false)
  (bind _asembercore_game_state_bp (cast `/Game/Embercore/EmbercoreGameState_BP` (`GameplayStatics.GetGameState`)))
  (bind _asdungeon_room (cast `DungeonRoom` (`self.GetOwner`)))
  (`/Game/Embercore/EmbercoreGameState_BP.OnStartRoom_Event` _asembercore_game_state_bp _asdungeon_room)
  (set `DungeonRoom.Active` true _asdungeon_room)
  (`self.K2_DestroyActor`))

(event `self.InteractableComponent_BP.OnStartTimerEvent`
  (`KismetSystemLibrary.PrintString` "Timer Start"))

(event `self.InteractableComponent_BP.OnUpdateTimerEvent`
  (params (IsHeld :type Boolean))
  (`KismetSystemLibrary.PrintString` (`KismetStringLibrary.Concat_StrStr` "Update Timer: " (`KismetStringLibrary.Conv_BoolToString` IsHeld))))

(event `self.InteractableComponent_BP.OnStopTimerEvent`
  (`KismetSystemLibrary.PrintString` "Stop"))

(event `self.InteractableComponent_BP.OnToggleInputEvent`
  (params (InToggle :type Boolean))
  (`KismetSystemLibrary.PrintString` (`KismetStringLibrary.Concat_StrStr` "Toggle Input: " (`KismetStringLibrary.Conv_BoolToString` InToggle))))

(fn `UserConstructionScript`)