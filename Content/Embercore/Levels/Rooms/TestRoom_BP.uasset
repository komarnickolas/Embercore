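; TestRoom_BP is a test room that builds its geometry on BeginPlay and reports when it has been cleared.
; It calls BuildRoom with a 5x5 layout and grid-material floor and wall meshes, then spawns a RoomStartTower_BP at half Width and Height.
; While Active, Tick polls the whole world for Enemy_BP actors.
; When none remain, it marks itself Cleared and inactive, then notifies EmbercoreGameState_BP through OnCompleteRoomEvent.
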(event `self.ReceiveBeginPlay`
  (`self.BuildRoom` 5 5 400.0 400.0 "/Game/StarterContent/Architecture/Floor_400x400.Floor_400x400" "/Engine/EngineMaterials/WorldGridMaterial.WorldGridMaterial" "/Game/StarterContent/Architecture/Wall_400x200.Wall_400x200" "/Engine/EngineMaterials/WorldGridMaterial.WorldGridMaterial")
  (`|SpawnActorFromClass` "/Game/Embercore/Levels/Rooms/RoomStartTower_BP.RoomStartTower_BP_C" (`KismetMathLibrary.MakeTransform` (`KismetMathLibrary.MakeVector` (`KismetMathLibrary.Conv_IntToDouble` (/ (`self.Width`) 2)) (`KismetMathLibrary.Conv_IntToDouble` (/ (`self.Height`) 2)) 50.0)) "Undefined" "OverrideRootScale" self null))

(event `self.ReceiveTick`
  (params (DeltaSeconds :type "Float (single-precision)"))
  (if (`self.Active`)
    (bind _outactors (`GameplayStatics.GetAllActorsOfClass` "/Game/Embercore/Enemies/Enemy/Enemy_BP.Enemy_BP_C"))
    (if (not (> (`KismetArrayLibrary.Array_Length` _outactors) 0))
      (set `self.Cleared` true)
      (set `self.Active` false)
      (bind _asembercore_game_state_bp (cast `/Game/Embercore/EmbercoreGameState_BP` (`GameplayStatics.GetGameState`)))
      (`/Game/Embercore/EmbercoreGameState_BP.OnCompleteRoom_Event` _asembercore_game_state_bp self))))

(fn `UserConstructionScript`)