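; Room_BP is a dungeon room actor that tracks whether it is active and cleared.
; Its construction script calls Fill, and BeginPlay spawns a RoomStartTower_BP, owned by the room, at the room's center.
; While Active, Tick polls every Enemy_BP in the world; when none remain it marks the room Cleared, deactivates it and reports completion to EmbercoreGameState_BP.
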(event `self.ReceiveBeginPlay`
  (bind _returnvalue (`self.GetCenter`))
  (`|SpawnActorFromClass` "/Game/Embercore/Levels/Dungeons/Rooms/RoomStartTower_BP.RoomStartTower_BP_C" (`KismetMathLibrary.MakeTransform` (`KismetMathLibrary.MakeVector` (.x _returnvalue) (.y _returnvalue) 50.0)) "Undefined" "OverrideRootScale" self null))

(event `self.ReceiveTick`
  (params (DeltaSeconds :type "Float (single-precision)"))
  (if (`self.Active`)
    (bind _outactors (`GameplayStatics.GetAllActorsOfClass` "/Game/Embercore/Enemies/Enemy/Enemy_BP.Enemy_BP_C"))
    (if (not (> (`KismetArrayLibrary.Array_Length` _outactors) 0))
      (set `self.Cleared` true)
      (set `self.Active` false)
      (bind _asembercore_game_state_bp (cast `/Game/Embercore/EmbercoreGameState_BP` (`GameplayStatics.GetGameState`)))
      (`/Game/Embercore/EmbercoreGameState_BP.OnCompleteRoom_Event` _asembercore_game_state_bp self))))

(fn `UserConstructionScript`
  (`self.Fill`))